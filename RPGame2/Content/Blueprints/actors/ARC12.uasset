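; ARC12 is an actor whose construction script applies the skeletal mesh currently stored in the custom game instance, along with its animation class.
; It reads CurrentMesh and CurrentAnimInstance from CustomGameInstance after running the parent construction script.
; A switch on the mesh asset's name sets a hardcoded relative scale and location for the Arc and Test ARC meshes, compensating for their differing sizes.
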(fn ConstructionScript
  (bind _mesh (Variables|Character|GetMesh))
  (bind _mesh_2 (Variables|Character|GetMesh))
  (bind _mesh_3 (Variables|Character|GetMesh))
  (|CallParentFunction)
  (bind _ascustom_game_instance (Utilities|Casting|CastToCustomGameInstance (Game|GetGameInstance)))
  (Class|SkinnedMeshComponent|SetSkeletalMesh _mesh (Variables|/Game/Blueprints/CustomGameInstance.CustomGameInstance_C|GetcurrentMesh _ascustom_game_instance) true)
  (Components|SkeletalMesh|SetAnimInstanceClass _mesh (Variables|/Game/Blueprints/CustomGameInstance.CustomGameInstance_C|GetcurrentAnimInstance _ascustom_game_instance))
  (switch name (Utilities|String|StringToName (Utilities|GetObjectName (Variables|/Game/Blueprints/CustomGameInstance.CustomGameInstance_C|GetcurrentMesh _ascustom_game_instance)))
    (:Arc
      (Transformation|SetRelativeScale3D _mesh_2 "60.000000,60.000000,60.000000")
      (Transformation|SetRelativeLocation _mesh_3 "0,0.000856,-132.000000" false false))
    (:TestARC
      (Transformation|SetRelativeScale3D _mesh_2 "0.250000,0.250000,0.250000")
      (Transformation|SetRelativeLocation _mesh_3 "0,0.000856,-95.000000" false false))))