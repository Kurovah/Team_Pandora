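; HintBlock is a hint trigger actor that shows a hint to the player and pauses the game.
; Any overlap with its Box writes HintTex to CurrentHint on the CustomGameInstance, then makes player 0's ARCChar HintWidget visible and sets HintOn.
; The overlapping actor is not checked, and the block contains no unpause logic.
; Tick slowly spins the Q and B components by a fixed per-frame step, independent of delta time.
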(event OnComponentBeginOverlap(Box)
  (params (OverlappedComponent :type Primitive%20Component%20Object%20Reference) (OtherActor :type Actor%20Object%20Reference) (OtherComp :type Primitive%20Component%20Object%20Reference) (OtherBodyIndex :type Integer) (bFromSweep :type Boolean) (SweepResult :type Hit%20Result%20Structure%20%28by%20ref%29))
  (bind _ascustom_game_instance (Utilities|Casting|CastToCustomGameInstance (Game|GetGameInstance)))
  (Variables|/Game/Blueprints/CustomGameInstance.CustomGameInstance_C|SetcurrentHint _ascustom_game_instance (Variables|Default|GetHintTex))
  (bind _asarcchar (Utilities|Casting|CastToARCChar (Game|Player|GetPlayerPawn 0)))
  (Widget|SetVisibility (Variables|/Game/Blueprints/actors/ARCChar.ARCChar_C|GetHintWidget _asarcchar) "Visible")
  (Variables|/Game/Blueprints/actors/ARCChar.ARCChar_C|SetHintOn _asarcchar true)
  (Game|SetGamePaused true))

(event EventTick
  (params (DeltaSeconds :type Float%20%28single-precision%29))
  (Transformation|AddRelativeRotation (Variables|Default|GetQ) "0,0.100000, 0" false false)
  (Transformation|AddRelativeRotation (Variables|Default|GetB) "0,0.100000, 0" false false))

(fn ConstructionScript)