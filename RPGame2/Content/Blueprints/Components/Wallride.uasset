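; Wallride component that gives the Player character wall slide and wall jump moves.
; Wallslide crosses the wall normal with capsule up and scales it by its dot with capsule forward, keeping velocity forward along the wall.
; It rotates the player to that direction and stores the rotation's success in ARCChar's WallRideActive.
; WallJump launches the player away from the wall and upward, then clears that flag.
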(event Custom|Wallslide
  (params (Wallnormal :type Vector))
  (bind _player (Variables|Default|GetPlayer))
  (bind _player_2 (Variables|Default|GetPlayer))
  (bind _dot_scale (Variables|Default|Getdot%20scale))
  (bind _player_3 (Variables|Default|GetPlayer))
  (bind _ws_scale (Variables|Default|Getws_scale))
  (bind _capsulecomponent (Variables|/Script/Engine.Character|GetCapsuleComponent _player_2))
  (bind _capsulecomponent_2 (Variables|/Script/Engine.Character|GetCapsuleComponent _player_3))
  (bind _returnvalue (Math|Vector|GetUpVector _capsulecomponent_2))
  (bind _returnvalue_2 (Math|Vector|GetForwardVector _capsulecomponent))
  (bind _returnvalue_3 (Math|Vector|CrossProduct Wallnormal _returnvalue))
  (bind _returnvalue_4 (Math|Vector|Normalize _returnvalue_3))
  (bind _returnvalue_5 (* _returnvalue_4 _ws_scale))
  (bind _returnvalue_6 (Math|Vector|DotProduct _returnvalue_5 _returnvalue_2))
  (bind _returnvalue_7 (* _dot_scale _returnvalue_6))
  (bind _returnvalue_8 (* _returnvalue_5 _returnvalue_7))
  (Variables|/Script/Engine.MovementComponent|SetVelocity (Variables|/Script/Engine.Character|GetCharacterMovement _player_3) _returnvalue_8)
  (bind _returnvalue_9 (Transformation|SetActorRotation _player (Math|Conversions|RotationFromXVector _returnvalue_8)))
  (bind _asarcchar (Utilities|Casting|CastToARCChar _player))
  (Variables|/Game/Blueprints/actors/ARCChar.ARCChar_C|SetwallRideActive _asarcchar _returnvalue_9))

(event Custom|WallJump
  (params (wallNormal :type Vector))
  (bind _player (Variables|Default|GetPlayer))
  (Character|LaunchCharacter _player (+ (* wallNormal (Variables|Default|Getwj_side_scale)) (* (Math|Vector|GetUpVector (Variables|/Script/Engine.Character|GetCapsuleComponent _player)) (Variables|Default|Getwj_up_scale))) false false)
  (bind _asarcchar (Utilities|Casting|CastToARCChar _player))
  (Variables|/Game/Blueprints/actors/ARCChar.ARCChar_C|SetwallRideActive _asarcchar false))