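; Actor component that gives the player a mid-air second jump.
; When tryJumpAgain is called and HasJump is set, it launches the character along its up and forward vectors, scaled by Upscale and ForwardScale, overriding only Z velocity.
; It then clears HasJump and plays the DoubleJump sound at the capsule; nothing in this file restores HasJump.
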(event Custom|tryJumpAgain
  (bind _player (Variables|Default|GetPlayer))
  (if (Variables|Default|GethasJump)
    (Character|LaunchCharacter _player (+ (* (Math|Vector|Normalize (Transformation|GetActorUpVector _player)) (Variables|Default|GetUpscale)) (* (Math|Vector|Normalize (Transformation|GetActorForwardVector _player)) (Variables|Default|GetForwardScale))) false true)
    (Variables|Default|SethasJump false)
    (Audio|PlaySoundatLocation "/Game/Sound_Effects/DoubleJump.DoubleJump" (Transformation|GetWorldLocation (Variables|/Script/Engine.Character|GetCapsuleComponent (Variables|Default|GetPlayer))) "0, 0, 0" 1.0 1.0 0.0 0 0 0)))