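; WallStick is a component that handles the player character's response to sticking to a wall and jumping off it.
; Begin_WallStick zeroes the movement velocity and turns the player to face into the wall, opposite the given normal.
; wallStickJump launches the player along the normal plus the capsule's up vector, each with its own scale, and rotates the player along the scaled normal.
; Wall detection is not in this graph, as both events receive the normal as input.
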(event Custom|Begin_WallStick
  (params (wallNorm :type Vector))
  (bind _player (Variables|Default|GetPlayer))
  (Variables|/Script/Engine.MovementComponent|SetVelocity (Variables|/Script/Engine.Character|GetCharacterMovement _player) "0, 0, 0")
  (Transformation|SetActorRotation _player (Math|Conversions|RotationFromXVector (* wallNorm -1.0))))

(event Custom|wallStickJump
  (params (wall%20norm :type Vector))
  (bind _player (Variables|Default|GetPlayer))
  (bind _wall_jump_side_scale (Variables|Default|Getwall%20jump%20side%20scale))
  (bind _returnvalue (* wall%20norm _wall_jump_side_scale))
  (Character|LaunchCharacter _player (+ _returnvalue (* (Math|Vector|GetUpVector (Variables|/Script/Engine.Character|GetCapsuleComponent _player)) (Variables|Default|Getwall%20jump%20up%20scale))) false false)
  (Transformation|SetActorRotation _player (Math|Conversions|RotationFromXVector _returnvalue)))